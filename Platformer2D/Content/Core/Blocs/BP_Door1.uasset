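; BP_Door1 is a level-exit door that works only while its Paper2D sprite is Active_door.
; When the player overlaps it, it disables input, clears IsPlaying on the game instance, plays a closing sound and a fade-out widget, then waits briefly.
; OpenNextLevel then uses the first false LevelStatus entry to mark progress and open a map from LevelNames, falling back to Start when that index is not above zero.
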(event EventBeginPlay)

(event Collision|EventActorBeginOverlap
  (params (OtherActor :type Actor%20Object%20Reference))
  (bind _asbp_player (Utilities|Casting|CastToBP_Player OtherActor))
  (if (== (Sprite|GetSprite (Actor|GetComponentbyClass self "/Script/Paper2D.PaperSpriteComponent")) "/Game/Assets/Sprite/Blocs/active_door.active_door")
    (Input|DisableInput _asbp_player 0)
    (bind _asbp_game_instance (Utilities|Casting|CastToBP_GameInstance (Game|GetGameInstance)))
    (Variables|/Game/Core/BP_GameInstance.BP_GameInstance_C|SetIsPlaying _asbp_game_instance false)
    (bind _returnvalue (UserInterface|CreateWidget "/Game/Widgets/WB_FadeOut.WB_FadeOut_C"))
    (UserInterface|Viewport|AddtoViewport _returnvalue 0)
    (Audio|PlaySound2D "/Game/Assets/SFX/door-close-79921.door-close-79921" 1.0 1.0 0.0 0 0)
    (Default|FadeAnim _returnvalue)
    (Utilities|FlowControl|Delay 2.0)
    (CallFunction|OpenNextLevel)))

(event EventTick
  (params (DeltaSeconds :type Float%20%28single-precision%29)))

(fn ConstructionScript)

(fn OpenNextLevel
  (bind _asbp_game_instance (Utilities|Casting|CastToBP_GameInstance (Game|GetGameInstance)))
  (Variables|Default|SetMapName (Utilities|Array|Get(acopy) (Variables|/Game/Core/BP_GameInstance.BP_GameInstance_C|GetLevelNames _asbp_game_instance) (Utilities|Array|FindItem (Variables|/Game/Core/BP_GameInstance.BP_GameInstance_C|GetLevelStatus _asbp_game_instance) false)))
  (if (> (Utilities|Array|FindItem (Variables|/Game/Core/BP_GameInstance.BP_GameInstance_C|GetLevelStatus _asbp_game_instance) false) 0)
    (Utilities|Array|SetArrayElem (Variables|/Game/Core/BP_GameInstance.BP_GameInstance_C|GetLevelStatus _asbp_game_instance) (Utilities|Array|FindItem (Variables|/Game/Core/BP_GameInstance.BP_GameInstance_C|GetLevelStatus _asbp_game_instance) false) true)
    (Game|OpenLevel(byName) (Variables|Default|GetMapName))
    (else
      (Game|OpenLevel(byName) "Start"))))