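; BP_BottomRightTornCable is a torn cable block whose electricity can kill the player.
; The cable counts as live while its PaperSprite shows one of a set of Top, Bottom, Left or Right sprite variants.
; Tick polls that sprite to switch the electricity flipbook between danger and idle.
; Box overlap repeats the check and calls PlayerDeath on the base, key-carrying or scotch-carrying player Blueprint.
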(event OnComponentBeginOverlap(Box)
  (params (OverlappedComponent :type Primitive%20Component%20Object%20Reference) (OtherActor :type Actor%20Object%20Reference) (OtherComp :type Primitive%20Component%20Object%20Reference) (OtherBodyIndex :type Integer) (bFromSweep :type Boolean) (SweepResult :type Hit%20Result%20Structure%20%28by%20ref%29))
  (bind _returnvalue (== 0 "/Game/Assets/Sprite/Blocs/bottom_bottomleft_Sprite.bottom_bottomleft_Sprite"))
  (bind _papersprite (Variables|Default|GetPaperSprite))
  (bind _returnvalue_2 (Sprite|GetSprite _papersprite))
  (bind _returnvalue_3 (== _returnvalue_2 "/Game/Assets/Sprite/Blocs/left_Sprite.left_Sprite"))
  (bind _returnvalue_4 (== _returnvalue_2 "/Game/Assets/Sprite/Blocs/left_topleft_Sprite.left_topleft_Sprite"))
  (bind _returnvalue_5 (== _returnvalue_2 "/Game/Assets/Sprite/Blocs/right_bottomright_Sprite.right_bottomright_Sprite"))
  (bind _returnvalue_6 (== _returnvalue_2 "/Game/Assets/Sprite/Blocs/right_Sprite.right_Sprite"))
  (bind _returnvalue_7 (== _returnvalue_2 "/Game/Assets/Sprite/Blocs/right_topright_Sprite.right_topright_Sprite"))
  (bind _returnvalue_8 (== _returnvalue_2 "/Game/Assets/Sprite/Blocs/top_Sprite.top_Sprite"))
  (bind _returnvalue_9 (== _returnvalue_2 "/Game/Assets/Sprite/Blocs/top_topleft_Sprite.top_topleft_Sprite"))
  (bind _returnvalue_10 (== _returnvalue_2 "/Game/Assets/Sprite/Blocs/top_topright_Sprite.top_topright_Sprite"))
  (bind _returnvalue_11 (== _returnvalue_2 "/Game/Assets/Sprite/Blocs/bottom_bottomright_Sprite.bottom_bottomright_Sprite"))
  (bind _returnvalue_12 (== _returnvalue_2 "/Game/Assets/Sprite/Blocs/bottom_Sprite.bottom_Sprite"))
  (bind _returnvalue_13 (== _returnvalue_2 "/Game/Assets/Sprite/Blocs/left_bottomleft_Sprite.left_bottomleft_Sprite"))
  (bind _returnvalue_14 (Math|Boolean|ORBoolean _returnvalue _returnvalue_11 _returnvalue_12))
  (bind _returnvalue_15 (Math|Boolean|ORBoolean _returnvalue_13 _returnvalue_3 _returnvalue_4))
  (bind _returnvalue_16 (Math|Boolean|ORBoolean _returnvalue_5 _returnvalue_6 _returnvalue_7))
  (bind _returnvalue_17 (Math|Boolean|ORBoolean _returnvalue_8 _returnvalue_9 _returnvalue_10))
  (bind _returnvalue_18 (Math|Boolean|ORBoolean _returnvalue_14 _returnvalue_15 _returnvalue_16 _returnvalue_17))
  (bind _asbp_player (Utilities|Casting|CastToBP_Player OtherActor)
    (:then
      (if _returnvalue_18
        (Default|PlayerDeath _asbp_player)))
    (:CastFailed
      (bind _asbp_player_with_key (Utilities|Casting|CastToBP_Player_With_Key OtherActor)
        (:then
          (if _returnvalue_18
            (Default|PlayerDeath _asbp_player_with_key)))
        (:CastFailed
          (bind _asbp_player_with_scotch (Utilities|Casting|CastToBP_Player_With_Scotch OtherActor))
          (if _returnvalue_18
            (Default|PlayerDeath _asbp_player_with_scotch)))))))

(event EventBeginPlay)

(event Collision|EventActorBeginOverlap
  (params (OtherActor :type Actor%20Object%20Reference)))

(event EventTick
  (params (DeltaSeconds :type Float%20%28single-precision%29))
  (bind _papersprite (Variables|Default|GetPaperSprite))
  (bind _returnvalue (Sprite|GetSprite _papersprite))
  (if (Math|Boolean|ORBoolean (Math|Boolean|ORBoolean (== 0 "/Game/Assets/Sprite/Blocs/bottom_bottomleft_Sprite.bottom_bottomleft_Sprite") (== _returnvalue "/Game/Assets/Sprite/Blocs/bottom_bottomright_Sprite.bottom_bottomright_Sprite") (== _returnvalue "/Game/Assets/Sprite/Blocs/bottom_Sprite.bottom_Sprite")) (Math|Boolean|ORBoolean (== _returnvalue "/Game/Assets/Sprite/Blocs/left_bottomleft_Sprite.left_bottomleft_Sprite") (== _returnvalue "/Game/Assets/Sprite/Blocs/left_Sprite.left_Sprite") (== _returnvalue "/Game/Assets/Sprite/Blocs/left_topleft_Sprite.left_topleft_Sprite")) (Math|Boolean|ORBoolean (== _returnvalue "/Game/Assets/Sprite/Blocs/right_bottomright_Sprite.right_bottomright_Sprite") (== _returnvalue "/Game/Assets/Sprite/Blocs/right_Sprite.right_Sprite") (== _returnvalue "/Game/Assets/Sprite/Blocs/right_topright_Sprite.right_topright_Sprite")) (Math|Boolean|ORBoolean (== _returnvalue "/Game/Assets/Sprite/Blocs/top_Sprite.top_Sprite") (== _returnvalue "/Game/Assets/Sprite/Blocs/top_topleft_Sprite.top_topleft_Sprite") (== _returnvalue "/Game/Assets/Sprite/Blocs/top_topright_Sprite.top_topright_Sprite")))
    (Sprite|SetFlipbook (Variables|Default|GetFB_Electricity) "/Game/Assets/Sprite/Electricity/FB_ElectricityDanger.FB_ElectricityDanger")
    (else
      (Sprite|SetFlipbook (Variables|Default|GetFB_Electricity) "/Game/Assets/Sprite/Electricity/FB_ElectricityIdle.FB_ElectricityIdle"))))

(fn ConstructionScript)