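; BP_Cadenas is a Paper2D padlock block that a player carrying a key unlocks on overlapping its box.
; If the sprite is still Cadenas_1, it replaces BP_Player_With_Key with a newly spawned, possessed BP_Player, removing the key.
; It then steps the sprite through to Cadenas_10 with short delays, playing a sound on early frames.
; The current sprite doubles as the locked state, so the unlock runs only once.
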(event OnComponentBeginOverlap(Box)
  (params (OverlappedComponent :type Primitive%20Component%20Object%20Reference) (OtherActor :type Actor%20Object%20Reference) (OtherComp :type Primitive%20Component%20Object%20Reference) (OtherBodyIndex :type Integer) (bFromSweep :type Boolean) (SweepResult :type Hit%20Result%20Structure%20%28by%20ref%29))
  (bind _self self)
  (bind _returnvalue (Actor|GetComponentbyClass _self "/Script/Paper2D.PaperSpriteComponent"))
  (bind _asbp_player_with_key (Utilities|Casting|CastToBP_Player_With_Key OtherActor))
  (if (== (Sprite|GetSprite (Actor|GetComponentbyClass self "/Script/Paper2D.PaperSpriteComponent")) "/Game/Assets/Sprite/Blocs/cadenas_1.cadenas_1")
    (Variables|Default|SetBP_Player_With_Key _asbp_player_with_key)
    (bind _returnvalue_2 (Game|SpawnActorfromClass "/Game/Core/BP_Player.BP_Player_C" (Transformation|GetActorTransform (Variables|Default|GetBP_Player_With_Key)) "AlwaysSpawn" "MultiplyWithRoot" 0 0))
    (Actor|DestroyActor (Variables|Default|GetBP_Player_With_Key))
    (Pawn|Possess (Game|GetPlayerController 0) _returnvalue_2)
    (Rendering|Components|Sprite|SetSprite _returnvalue "/Game/Assets/Sprite/Blocs/cadenas_2.cadenas_2")
    (Audio|PlaySound2D "/Game/Core/Sounds/cadenas.cadenas" 1.0 1.0 0.0 0 0)
    (Utilities|FlowControl|Delay 0.1)
    (Rendering|Components|Sprite|SetSprite _returnvalue "/Game/Assets/Sprite/Blocs/cadenas_3.cadenas_3")
    (Audio|PlaySound2D "/Game/Core/Sounds/cadenas.cadenas" 1.0 1.0 0.0 0 0)
    (Utilities|FlowControl|Delay 0.1)
    (Rendering|Components|Sprite|SetSprite _returnvalue "/Game/Assets/Sprite/Blocs/cadenas_4.cadenas_4")
    (Audio|PlaySound2D "/Game/Core/Sounds/cadenas.cadenas" 1.0 1.0 0.0 0 0)
    (Utilities|FlowControl|Delay 0.1)
    (Rendering|Components|Sprite|SetSprite _returnvalue "/Game/Assets/Sprite/Blocs/cadenas_5.cadenas_5")
    (Audio|PlaySound2D "/Game/Core/Sounds/cadenas.cadenas" 1.0 1.0 0.0 0 0)
    (Utilities|FlowControl|Delay 0.1)
    (Rendering|Components|Sprite|SetSprite _returnvalue "/Game/Assets/Sprite/Blocs/cadenas_6.cadenas_6")
    (Utilities|FlowControl|Delay 0.1)
    (Rendering|Components|Sprite|SetSprite _returnvalue "/Game/Assets/Sprite/Blocs/cadenas_7.cadenas_7")
    (Utilities|FlowControl|Delay 0.1)
    (Rendering|Components|Sprite|SetSprite _returnvalue "/Game/Assets/Sprite/Blocs/cadenas_8.cadenas_8")
    (Utilities|FlowControl|Delay 0.1)
    (Rendering|Components|Sprite|SetSprite _returnvalue "/Game/Assets/Sprite/Blocs/cadenas_9.cadenas_9")
    (Utilities|FlowControl|Delay 0.1)
    (Rendering|Components|Sprite|SetSprite _returnvalue "/Game/Assets/Sprite/Blocs/cadenas_10.cadenas_10")))

(event EventBeginPlay)

(event Collision|EventActorBeginOverlap
  (params (OtherActor :type Actor%20Object%20Reference)))

(event EventTick
  (params (DeltaSeconds :type Float%20%28single-precision%29)))

(fn ConstructionScript)