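; BP_KeyBlock is a block that gives the player a key when BP_Player overlaps its Box.
; It replaces itself with a BP_YellowBlock at the same transform.
; It also swaps the player pawn for a BP_Player_With_Key, possessed by player controller 0, and plays the Interact sound.
; BeginPlay enables the Box's query and physics collision only after a short delay.
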(event OnComponentBeginOverlap(Box)
  (params (OverlappedComponent :type Primitive%20Component%20Object%20Reference) (OtherActor :type Actor%20Object%20Reference) (OtherComp :type Primitive%20Component%20Object%20Reference) (OtherBodyIndex :type Integer) (bFromSweep :type Boolean) (SweepResult :type Hit%20Result%20Structure%20%28by%20ref%29))
  (bind _self self)
  (bind _asbp_player (Utilities|Casting|CastToBP_Player OtherActor))
  (Utilities|FlowControl|Sequence
    (:then_0
      (Game|SpawnActorfromClass "/Game/Core/Blocs/BP_YellowBlock.BP_YellowBlock_C" (Transformation|GetActorTransform _self) "Undefined" "MultiplyWithRoot" 0 0)
      (Actor|DestroyActor _self))
    (:then_1
      (Variables|Default|SetPlayer _asbp_player)
      (bind _returnvalue (Game|SpawnActorfromClass "/Game/Core/BP_Player_With_Key.BP_Player_With_Key_C" (Transformation|GetActorTransform (Variables|Default|GetPlayer)) "AlwaysSpawn" "MultiplyWithRoot" 0 0))
      (Actor|DestroyActor (Variables|Default|GetPlayer))
      (Pawn|Possess (Game|GetPlayerController 0) _returnvalue)
      (Audio|PlaySound2D "/Game/Core/Sounds/interact.interact" 1.0 1.0 0.0 0 0))))

(event Collision|EventActorBeginOverlap
  (params (OtherActor :type Actor%20Object%20Reference)))

(event EventTick
  (params (DeltaSeconds :type Float%20%28single-precision%29)))

(event EventBeginPlay
  (Utilities|FlowControl|Delay 3.0)
  (Collision|SetCollisionEnabled (Variables|Default|GetBox) "QueryAndPhysics"))

(fn ConstructionScript)