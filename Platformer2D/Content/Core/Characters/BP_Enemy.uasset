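; Paper2D patrolling enemy that kills the player on capsule contact and dies when its head collider is hit.
; MoveForward drives walking, while wall and ledge overlap triggers flip its rotation.
; Enemy collisions either turn it around or pause it first, based on both facing directions.
; Head hits add score and play a timed death sequence before destruction; Tick halts movement when game-instance play ends, including after player death.
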(event OnComponentEndOverlap(LedgeDetectorCollider)
  (params (OverlappedComponent :type Primitive%20Component%20Object%20Reference) (OtherActor :type Actor%20Object%20Reference) (OtherComp :type Primitive%20Component%20Object%20Reference) (OtherBodyIndex :type Integer))
  ;[1 1 1] Ledge Detection
  (CallFunction|TurnCharacter))

(event OnComponentHit(CapsuleComponent)
  (params (HitComponent :type Primitive%20Component%20Object%20Reference) (OtherActor :type Actor%20Object%20Reference) (OtherComp :type Primitive%20Component%20Object%20Reference) (NormalImpulse :type Vector :default "0, 0, 0") (Hit :type Hit%20Result%20Structure%20%28by%20ref%29))
  (bind _charactermovement (Variables|Character|GetCharacterMovement))
  (bind _sprite (Variables|Default|GetSprite))
  ;[1 1 1] Hit Detection of other characters (Player and AI)
  (Utilities|FlowControl|Sequence
    (:then_0
      (bind _asbp_player (Utilities|Casting|CastToBP_Player OtherActor))
      (if (not (Variables|Default|GetIsPlayerDead))
        (Variables|Default|SetIsPlayerDead true)
        (Default|PlayerDeath _asbp_player)))
    (:then_1
      ;[1 1 1] Enemy Detection
      (bind _asbp_enemy (Utilities|Casting|CastToBP_Enemy OtherActor))
      (if (== (+ (Class|KismetMathLibrary|ToInt64(Float) (.x (Transformation|GetActorForwardVector _asbp_enemy))) (Class|KismetMathLibrary|ToInt64(Float) (.x (Transformation|GetActorForwardVector self)))) 1)
        (Variables|/Script/Engine.CharacterMovementComponent|SetMaxWalkSpeed _charactermovement 0.0)
        (Sprite|SetFlipbook _sprite "/Game/Assets/Sprite/EnemyAnimation/Idle/FB_EnemyIdle.FB_EnemyIdle")
        (Utilities|FlowControl|Delay 2.0)
        (if (not (Variables|Default|GetIsEnemyDead))
          (CallFunction|TurnCharacter)
          (Variables|/Script/Engine.CharacterMovementComponent|SetMaxWalkSpeed _charactermovement 3e+02)
          (Sprite|SetFlipbook _sprite "/Game/Assets/Sprite/EnemyAnimation/Walking/FB_EnemyWalk.FB_EnemyWalk")
          (Utilities|FlowControl|Delay 2.0))
        (else
          (CallFunction|TurnCharacter))))))

(event OnComponentBeginOverlap(WallDetectionCollider)
  (params (OverlappedComponent :type Primitive%20Component%20Object%20Reference) (OtherActor :type Actor%20Object%20Reference) (OtherComp :type Primitive%20Component%20Object%20Reference) (OtherBodyIndex :type Integer) (bFromSweep :type Boolean) (SweepResult :type Hit%20Result%20Structure%20%28by%20ref%29))
  ;[1 1 1] Wall Detection
  (CallFunction|TurnCharacter))

(event OnComponentHit(DeathDetectionCollision)
  (params (HitComponent :type Primitive%20Component%20Object%20Reference) (OtherActor :type Actor%20Object%20Reference) (OtherComp :type Primitive%20Component%20Object%20Reference) (NormalImpulse :type Vector :default "0, 0, 0") (Hit :type Hit%20Result%20Structure%20%28by%20ref%29))
  ;[1 1 1] Death Detection (Player jumps on head)
  (Utilities|FlowControl|Sequence
    (:then_0
      (bind _asbp_game_instance (Utilities|Casting|CastToBP_GameInstance (Game|GetGameInstance)))
      (Variables|/Game/Core/BP_GameInstance.BP_GameInstance_C|SetScore _asbp_game_instance (+ (Variables|/Game/Core/BP_GameInstance.BP_GameInstance_C|GetScore _asbp_game_instance) 20))
      (CallFunction|EnemyDeathAnimation)
      (Utilities|FlowControl|Delay 1.0)
      (CallFunction|SetDeadEnemy)
      (Utilities|FlowControl|Delay 1.0)
      (CallFunction|DestroyEnemy))))

(event Custom|MoveForward
  ;[1 1 1] AI Movement
  (Pawn|Input|AddMovementInput (Transformation|GetActorForwardVector) 1.0 false)
  (Variables|Default|SetMax%20Walk%20Speed 3e+02))

(event EventTick
  (params (DeltaSeconds :type Float%20%28single-precision%29))
  (bind _asbp_game_instance (Utilities|Casting|CastToBP_GameInstance (Game|GetGameInstance)))
  (Utilities|FlowControl|Sequence
    (:then_0
      (if (Variables|Default|GetIsPlayerDead)
        (Variables|/Game/Core/BP_GameInstance.BP_GameInstance_C|SetIsPlaying _asbp_game_instance false)))
    (:then_1
      (if (not (Variables|/Game/Core/BP_GameInstance.BP_GameInstance_C|GetIsPlaying _asbp_game_instance))
        (Pawn|Components|CharacterMovement|DisableMovement (Variables|Character|GetCharacterMovement))
        (Sprite|SetFlipbook (Variables|Default|GetSprite) "/Game/Assets/Sprite/EnemyAnimation/Idle/FB_EnemyIdle.FB_EnemyIdle")))))

(fn ConstructionScript)

(fn TurnCharacter
  (Transformation|SetActorRotation (Math|Rotator|CombineRotators (Transformation|GetActorRotation) "0.000000,180.000000,0.000000")))

(fn DestroyEnemy
  (Actor|DestroyActor))

(fn EnemyDeathAnimation
  (Variables|Default|SetIsEnemyDead true)
  (Components|DestroyComponent (Variables|Collision|GetCapsuleComponent))
  (Variables|/Script/Engine.CharacterMovementComponent|SetMaxCustomMovementSpeed (Variables|Character|GetCharacterMovement) 0.0)
  (Input|DisableInput 0)
  (Sprite|SetFlipbook (Variables|Default|GetSprite) "/Game/Assets/Sprite/EnemyAnimation/Death/FB_DyingRobotBig.FB_DyingRobotBig"))

(fn SetDeadEnemy
  (Sprite|SetFlipbook (Variables|Default|GetSprite) "/Game/Assets/Sprite/EnemyAnimation/Death/FB_DeadRobotBig.FB_DeadRobotBig"))