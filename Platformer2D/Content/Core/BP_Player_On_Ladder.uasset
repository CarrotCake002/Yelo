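; Player pawn used while climbing ladders in a side-view flipbook game, moving in flying mode.
; Up and MoveRight input moves it while inside the box bounds of any BP_Ladder or BP_SideLadder, scanned from all such actors on each axis event.
; Leaving every ladder or pressing Jump spawns BP_Player in place, possesses it and destroys this pawn.
; Tick swaps the climb/idle flipbook by vertical velocity and plays climb sounds on alternating frames.
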(event EventBeginPlay)

(event Collision|EventActorBeginOverlap
  (params (OtherActor :type Actor%20Object%20Reference)))

(event EventTick
  (params (DeltaSeconds :type Float%20%28single-precision%29))
  (Utilities|FlowControl|Sequence
    (:then_0
      (if (== (.Z (Math|Vector|BreakVector (Transformation|GetVelocity))) 0.0)
        (Sprite|SetFlipbook (Variables|Default|GetSprite) "/Game/Assets/Sprite/PlayerAnimation/Ladder/PFB_ladder_inactive.PFB_ladder_inactive")
        (else
          (Sprite|SetFlipbook (Variables|Default|GetSprite) "/Game/Assets/Sprite/PlayerAnimation/Ladder/PFB_ladder.PFB_ladder"))))
    (:then_1
      (if (== (Class|PaperFlipbookComponent|GetFlipbook (Variables|Default|GetSprite)) "/Game/Assets/Sprite/PlayerAnimation/Ladder/PFB_ladder.PFB_ladder")
        (if (or (== (Class|PaperFlipbookComponent|GetPlaybackPositioninFrames (Variables|Default|GetSprite)) (Variables|Default|GetClimbValue)) false)
          (Utilities|FlowControl|DoOnce false :!label _label
            (:Completed
              (Variables|Default|SetClimbValue (Class|KismetMathLibrary|PercentInt64Int64 (+ (Variables|Default|GetClimbValue) 2) 5))
              (Audio|PlaySound2D "/Game/Core/Sounds/MS_ladder.MS_ladder" 1.0 1.0 0.0 0 0)))
          (else
            (goto _label Reset)))))))

(event Input|ActionEvents|InputActionJump
  (params (Key :type Key%20Structure :default "None"))
  ;[1 1 1] Jump (cancel ladder)
  (:Pressed
    (Character|Jump)
    (bind _returnvalue (Game|SpawnActorfromClass "/Game/Core/BP_Player.BP_Player_C" (Transformation|GetActorTransform) "AlwaysSpawn" "MultiplyWithRoot" 0 0))
    (Pawn|Possess (Pawn|GetController) _returnvalue)
    (Actor|DestroyActor)))

(event Input|AxisEvents|InputAxisMoveRight
  (params (AxisValue :type Float%20%28single-precision%29))
  ;[1 1 1] Movement right and left
  (Variables|Default|SetClimbing false)
  (bind _outactors (Actor|GetAllActorsOfClass "/Game/Core/Blocs/BP_Ladder.BP_Ladder_C"))
  (for _array_element _outactors
    (bind _isplayerinside (CallFunction|IsPlayerInside (.Origin (Collision|GetActorBounds _array_element false false)) 72 72))
    (if _isplayerinside
      (Variables|Default|SetClimbing true)
      (Pawn|Input|AddMovementInput (Transformation|GetActorForwardVector) (/ AxisValue 2.0) false)))
  (bind _outactors_2 (Actor|GetAllActorsOfClass "/Game/Core/Blocs/BP_SideLadder.BP_SideLadder_C"))
  (for _array_element_2 _outactors_2
    (bind _isplayerinside_2 (CallFunction|IsPlayerInside (.Origin (Collision|GetActorBounds _array_element_2 false false)) 52 72))
    (if _isplayerinside_2
      (Variables|Default|SetClimbing true)
      (Pawn|Input|AddMovementInput (Transformation|GetActorForwardVector) (/ AxisValue 2.0) false)))
  (if (not (Variables|Default|GetClimbing))
    ;[1 1 1] sGo back to BP_Player
    (bind _returnvalue (Game|SpawnActorfromClass "/Game/Core/BP_Player.BP_Player_C" (Transformation|GetActorTransform) "AlwaysSpawn" "MultiplyWithRoot" 0 0))
    (Pawn|Possess (Game|GetPlayerController 0) _returnvalue)
    (Actor|DestroyActor)))

(event Input|AxisEvents|InputAxisUp
  (params (AxisValue :type Float%20%28single-precision%29))
  (Variables|Default|SetClimbing false)
  ;[1 1 1] Climb Ladder
  (bind _outactors (Actor|GetAllActorsOfClass "/Game/Core/Blocs/BP_Ladder.BP_Ladder_C"))
  (for _array_element _outactors
    (bind _isplayerinside (CallFunction|IsPlayerInside (.Origin (Collision|GetActorBounds _array_element false false)) 72 72))
    (if _isplayerinside
      (Variables|Default|SetClimbing true)
      (Pawn|Input|AddMovementInput "0.000000,0.000000,0.500000" AxisValue false)))
  (if (not (Variables|Default|GetClimbing))
    ;[1 1 1] Climb Side Ladder
    (bind _outactors_2 (Actor|GetAllActorsOfClass "/Game/Core/Blocs/BP_SideLadder.BP_SideLadder_C"))
    (for _array_element_2 _outactors_2
      (bind _isplayerinside_2 (CallFunction|IsPlayerInside (.Origin (Collision|GetActorBounds _array_element_2 false false)) 52 72))
      (if _isplayerinside_2
        (Variables|Default|SetClimbing true)
        (Pawn|Input|AddMovementInput "0.000000,0.000000,0.500000" AxisValue false)))
    (if (not (Variables|Default|GetClimbing))
      ;[1 1 1] sGo back to BP_Player
      (bind _returnvalue (Game|SpawnActorfromClass "/Game/Core/BP_Player.BP_Player_C" (Transformation|GetActorTransform) "AlwaysSpawn" "MultiplyWithRoot" 0 0))
      (Pawn|Possess (Game|GetPlayerController 0) _returnvalue)
      (Actor|DestroyActor))))

(fn ConstructionScript
  (Pawn|Components|CharacterMovement|SetMovementMode (Variables|Character|GetCharacterMovement) "MOVE_Flying" 0)
  (Variables|Default|SetClimbValue 2))

(fn IsPlayerInside
  (params (Origin :type Vector) (Size%20block%20X :type Integer) (Size%20block%20Z :type Integer))
  (bind _returnvalue (Transformation|GetActorLocation))
  (bind (_x _y _z) (Math|Vector|BreakVector Origin))
  (bind (_x_2 _y_2 _z_2) (Math|Vector|BreakVector Origin))
  (bind _returnvalue_2 (/ Size%20block%20X 2))
  (bind (_x_3 _y_3 _z_3) (Math|Vector|BreakVector _returnvalue))
  (if (<= _x_3 (+ _x_2 _returnvalue_2))
    (if (<= _z_3 (+ _z Size%20block%20Z))
      (if (> _x_3 (- _x _returnvalue_2))
        (if (> _z_3 _z_2)
          (return true)
          (else
            (return false)))
        (else
          (return false)))
      (else
        (return false)))
    (else
      (return false))))